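; RBP is a clickable red star sprite actor that adds to a red score when clicked.
; On BeginPlay it picks a random Y/Z endpoint on a fixed X plane and plays a timeline that lerps from its current, continually updated location toward it.
; Clicking RSprite calls the Plusredscore dispatcher and destroys the actor.
; Debug prints report the click and the location when movement finishes.
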(event OnClicked(RSprite)
  (params (TouchedComponent :type Primitive%20Component%20Object%20Reference))
  (Development|PrintString "Click on Red Star ")
  (Default|CallPlusredscore)
  (Actor|DestroyActor))

(event EventBeginPlay
  (bind _self self)
  (bind _returnvalue (Transformation|GetActorLocation _self))
  (bind _output_get (Variables|Default|Setendpoint (Math|Vector|MakeVector 1e+01 (Math|Random|RandomFloatinRange -2.4e+02 2.4e+02) (Math|Random|RandomFloatinRange 6e+01 2.7e+02))))
  (bind _alpha (Timeline|Timeline_0 Play)
    (:Update
      (Transformation|SetActorLocation _self (Math|Vector|Lerp(Vector) _returnvalue _output_get _alpha) false false))
    (:Finished
      (Development|PrintString (Utilities|String|Append "redmove" (Utilities|String|ToString(Vector) _returnvalue))))))

(event EventActorBeginOverlap
  (params (OtherActor :type Actor%20Object%20Reference)))

(event EventTick
  (params (DeltaSeconds :type Float%20%28single-precision%29)))

(fn ConstructionScript)
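; Clickable blue star sprite actor that drifts toward a random point and adds to the blue score when clicked.
; BeginPlay picks the target at a fixed X with random Y and Z.
; A Delay on Tick throttles movement to roughly one-second steps, each covering a third of the remaining distance until a counter passes its limit.
; Clicking the sprite prints a message, calls Plusbluescore and destroys the actor.
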(event OnClicked(NewPaperSprite)
  (params (TouchedComponent :type Primitive%20Component%20Object%20Reference))
  (Development|PrintText "Click on Blue Star ")
  (Default|CallPlusbluescore)
  (Actor|DestroyActor))

(event EventBeginPlay
  (bind _output_get (Variables|Default|Setp (Math|Vector|MakeVector 1e+01 (Math|Random|RandomFloatinRange -2.4e+02 2.4e+02) (Math|Random|RandomFloatinRange 6e+01 2.7e+02)))))

(event EventActorBeginOverlap
  (params (OtherActor :type Actor%20Object%20Reference)))

(event EventTick
  (params (DeltaSeconds :type Float%20%28single-precision%29))
  (bind _self self)
  (Utilities|FlowControl|Delay 1.0)
  (if (<= (Variables|Default|Getc) 3)
    (Variables|Default|Setc (+ (Variables|Default|Getc) 1))
    (Transformation|AddActorWorldOffset _self (/ (- (stale EventBeginPlay _output_get) (Transformation|GetActorLocation _self)) 3))
    (Development|PrintString "move")))

(fn ConstructionScript)